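; NPC character Blueprint for a pedestrian-like NPC that switches between walking and running away when the player attacks.
; Tick polls the Spawner's attack flag, swaps walk speed on each change and forwards the state toggle to its NPC_AI controller.
; A FirstPersonProjectile hit kills the NPC, ragdolls its mesh, disables movement and reports the attack to the Spawner.
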(event Custom|EventChangeState)

(event EventBeginPlay
  (bind _charactermovement (Variables|Character|GetCharacterMovement))
  ;[1 1 1] Inicialitzar
  (Variables|Default|SetAIControllerClass "/Game/NPC/Scripts/NPC_AI.NPC_AI_C")
  (bind _asnpc_ai (Utilities|Casting|CastToNPC_AI (AI|GetAIController self)))
  (Variables|Default|SetAI _asnpc_ai)
  (bind _output_get (Variables|Default|SetisRunningAway false))
  (if _output_get
    (Variables|/Script/Engine.CharacterMovementComponent|SetMaxWalkSpeed _charactermovement 4.5e+02)
    (else
      (Variables|/Script/Engine.CharacterMovementComponent|SetMaxWalkSpeed _charactermovement 1.5e+02))))

(event EventTick
  (params (DeltaSeconds :type Float%20%28single-precision%29))
  (bind _charactermovement (Variables|Character|GetCharacterMovement))
  ;[1 1 1] Decidir velocitat
  (if (Variables|/Game/NPC/Scripts/NPC_Spawner.NPC_Spawner_C|GetisPlayerAttacking (Variables|Default|GetSpawner))
    (if (not (Variables|Default|GetisRunningAway))
      (Variables|/Script/Engine.CharacterMovementComponent|SetMaxWalkSpeed _charactermovement 4.5e+02)
      (Variables|Default|SetisRunningAway (not (Variables|Default|GetisRunningAway)) :!label _label)
      (CallFunction|EventChangeState)
      (Default|EventChangeState (Variables|Default|GetAI)))
    (elif (Variables|Default|GetisRunningAway)
      (Variables|/Script/Engine.CharacterMovementComponent|SetMaxWalkSpeed _charactermovement 1.5e+02)
      (goto _label))))

(event Collision|EventHit
  (params (MyComp :type Primitive%20Component%20Object%20Reference) (Other :type Actor%20Object%20Reference) (OtherComp :type Primitive%20Component%20Object%20Reference) (bSelfMoved :type Boolean) (HitLocation :type Vector :default "0, 0, 0") (HitNormal :type Vector :default "0, 0, 0") (NormalImpulse :type Vector :default "0, 0, 0") (Hit :type Hit%20Result%20Structure%20%28by%20ref%29))
  ;[1 1 1] Morir
  (Utilities|Casting|CastToFirstPersonProjectile Other)
  (Variables|Default|SetisAlive false)
  (Physics|SetSimulatePhysics (Variables|Character|GetMesh) true)
  (Pawn|Components|CharacterMovement|DisableMovement (Variables|Character|GetCharacterMovement))
  (Default|EventPlayerAttack (Variables|Default|GetSpawner)))

(fn ConstructionScript)