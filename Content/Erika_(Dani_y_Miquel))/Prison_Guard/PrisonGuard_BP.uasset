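; Prison guard actor that sleeps leaning with sleeping audio and carries keys until it is killed.
; Its Die event removes the capsule and keys, plays a forward-fall death animation, stops the sleeping sound and, after a short delay, plays a key pickup sound.
; Die then records the time of death, which Tick checks to destroy the actor fifteen seconds later.
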(event Custom|Die
  (Components|DestroyComponent (Variables|Default|GetCapsule))
  (Components|DestroyComponent (Variables|Default|GetKeys))
  (Components|Animation|PlayAnimation (Variables|Default|GetGuard) "/Game/Erika_(Dani_y_Miquel))/Prison_Guard/Falling_Forward_Death.Falling_Forward_Death" false)
  (Audio|Components|Audio|Stop (stale EventBeginPlay _returnvalue))
  (Utilities|FlowControl|Delay 0.7)
  (Audio|PlaySoundatLocation "/Game/Erika_(Dani_y_Miquel))/Prison_Guard/PickUpKeys.PickUpKeys" (Transformation|GetWorldLocation (Variables|Default|GetDefaultSceneRoot)) "0, 0, 0" 1.0 1.0 0.0 0 0 0)
  (Variables|Default|SetTimeKilled (Utilities|Time|GetGameTimeinSeconds)))

(event EventBeginPlay
  (Components|Animation|PlayAnimation (Variables|Default|GetGuard) "/Game/Erika_(Dani_y_Miquel))/Prison_Guard/Leaning.Leaning" true)
  (bind _returnvalue (Audio|SpawnSoundatLocation "/Game/Erika_(Dani_y_Miquel))/Prison_Guard/full_sleeping_SC.full_sleeping_SC" (Transformation|GetWorldLocation (Variables|Default|GetDefaultSceneRoot)) "0, 0, 0" 1.0 1.0 0.0 0 0 false)))

(event EventTick
  (params (DeltaSeconds :type Float%20%28single-precision%29))
  (if (!= (Variables|Default|GetTimeKilled) -1.0)
    (if (>= (- (Utilities|Time|GetGameTimeinSeconds) (Variables|Default|GetTimeKilled)) 15.0)
      (Actor|DestroyActor))))

(fn ConstructionScript)