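; BP_Crypt_Doorway is a crypt double door that sends the first-person player to the town level when they enter its trigger box.
; The overlap plays a timeline that swings both door meshes open in mirrored yaw.
; Each timeline update also saves the arrow count to the Singleton game instance, creates a loading-screen widget and reaches a short delay before opening the level.
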(event OnComponentBeginOverlap(Box)
  (params (OverlappedComponent :type Primitive%20Component%20Object%20Reference) (OtherActor :type Actor%20Object%20Reference) (OtherComp :type Primitive%20Component%20Object%20Reference) (OtherBodyIndex :type Integer) (bFromSweep :type Boolean) (SweepResult :type Hit%20Result%20Structure%20%28by%20ref%29))
  (bind _asbp_first_person (Utilities|Casting|CastToBP_FirstPerson OtherActor))
  (bind _doortimer (Timeline|doortimer Play)
    (:Update
      (Utilities|FlowControl|Sequence
        (:then_0
          (Transformation|SetRelativeRotation (Variables|Default|GetSM_DoorWay_Large_Door_Right) (Math|Rotator|MakeRotator 0.0 0.0 (+ _doortimer -9e+01)) false false)
          (bind _assingleton (Utilities|Casting|CastToSingleton (Game|GetGameInstance)))
          (Default|SetNumArrows _assingleton (Variables|/Game/Erika_(Dani_y_Miquel))/BP/BP_FirstPerson.BP_FirstPerson_C|GetNumArrows _asbp_first_person))
          (bind _returnvalue (UserInterface|CreateWidget "/Game/Quim/Menus/LoadingScreen_Widget.LoadingScreen_Widget_C"))
          (UserInterface|Viewport|AddtoViewport _returnvalue 0)
          (Utilities|FlowControl|Delay 0.2)
          (Game|OpenLevel(byObjectReference) "/Game/Denís/Escenario/TownLevel_con_modelos_y_suelo.TownLevel_con_modelos_y_suelo"))
        (:then_1
          (Transformation|SetRelativeRotation (Variables|Default|GetSM_DoorWay_Large_Door_Left) (Math|Rotator|MakeRotator 0.0 0.0 (+ (* -1 _doortimer) -9e+01)) false false))))))

(event EventBeginPlay)

(event Collision|EventActorBeginOverlap
  (params (OtherActor :type Actor%20Object%20Reference)))

(event EventTick
  (params (DeltaSeconds :type Float%20%28single-precision%29)))

(fn ConstructionScript)