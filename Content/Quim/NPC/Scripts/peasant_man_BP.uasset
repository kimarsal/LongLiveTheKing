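; Peasant man NPC Blueprint that links the character to its animation Blueprint.
; On BeginPlay it calls the parent, casts the mesh's anim instance to peasant_man_ABP and caches it.
; EventChangeState forwards the state change to that animation Blueprint.
; Tick and overlap events are disabled, and the construction script only calls the parent.
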(event Custom|EventChangeState
  (Default|EventChangeState (Variables|Default|GetABP)))

(event EventBeginPlay
  (|CallParentFunction)
  (bind _aspeasant_man_abp (Utilities|Casting|CastTopeasant_man_ABP (Components|SkeletalMesh|GetAnimInstance (Variables|Character|GetMesh))))
  (Variables|Default|SetABP _aspeasant_man_abp))

(event Collision|EventActorBeginOverlap
  (params (OtherActor :type Actor%20Object%20Reference)))

(event EventTick
  (params (DeltaSeconds :type Float%20%28single-precision%29))
  (|CallParentFunction DeltaSeconds) ; This node is disabled and will not be called.\nDrag off pins to build functionality.
)

(fn ConstructionScript
  (|CallParentFunction))