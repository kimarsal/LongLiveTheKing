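; YBot_BP is a peasant NPC Blueprint for the YBot that links the NPC to its animation Blueprint.
; On BeginPlay it runs the parent logic, then casts the mesh's anim instance to YBot_ABP and stores the reference.
; EventChangeState forwards state changes to that animation Blueprint, while Tick and overlap events are disabled.
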(event Custom|EventChangeState
  (Default|EventChangeState (Variables|Default|GetABP_0)))

(event EventBeginPlay
  (|CallParentFunction)
  (bind _asybot_abp (Utilities|Casting|CastToYBot_ABP (Components|SkeletalMesh|GetAnimInstance (Variables|Character|GetMesh))))
  (Variables|Default|SetABP_0 _asybot_abp))

(event Collision|EventActorBeginOverlap
  (params (OtherActor :type Actor%20Object%20Reference)))

(event EventTick
  (params (DeltaSeconds :type Float%20%28single-precision%29))
  (|CallParentFunction DeltaSeconds) ; This node is disabled and will not be called.\nDrag off pins to build functionality.
)

(fn ConstructionScript
  (|CallParentFunction))